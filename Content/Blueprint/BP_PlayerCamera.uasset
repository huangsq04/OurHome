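; BP_PlayerCamera is a player camera for picking and moving to points on a planet with the mouse cursor.
; DClick traces from the cursor, using a MultiGate with a short delayed reset to separate single from double clicks.
; A first hit debug-draws and prints PlanetActor's terrain data.
; A quick second hit calls MovePoint with a position offset above the terrain height along the origin-to-hit direction.
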(event EventBeginPlay
  (Variables|/Script/Engine.PlayerController|SetbShowMouseCursor (Game|GetPlayerController 0) true)
  (Class|PlayerCameraPawn|SetUsingAbsoluteRotation (Variables|Default|GetStaticMesh) true))

(event Collision|EventActorBeginOverlap
  (params (OtherActor :type Actor%20Object%20Reference)))

(event EventTick
  (params (DeltaSeconds :type Float%20%28single-precision%29)))

(event Input|ActionEvents|InputActionDClick
  (params (Key :type Key%20Structure :default "None"))
  (bind _returnvalue (Game|GetPlayerController 0))
  (bind _returnvalue_2 (Game|GetPlayerController 0))
  (bind _planetactor (Variables|Default|GetPlanetActor))
  (bind (_worldlocation _worlddirection) (Game|Player|ConvertMouseLocationToWorldSpace _returnvalue))
  (bind (_worldlocation_2 _worlddirection_2) (Game|Player|ConvertMouseLocationToWorldSpace _returnvalue_2))
  (:Pressed
    (Utilities|FlowControl|MultiGate false false -1 :!label _label
      (:Out%200
        (bind _outhit (Collision|LineTraceByChannel _worldlocation (+ _worldlocation (* _worlddirection (Math|Vector|VectorLength _worldlocation))) "TraceTypeQuery1" false 0 "None"))
        (if (.bBlockingHit (Collision|BreakHitResult _outhit))
          (bind _returnvalue_3 (Class|PlanetActor|GetTerrainPosition _planetactor (Math|Vector|Normalize (.ImpactPoint (Collision|BreakHitResult _outhit)) 1e-06)))
          (Rendering|Debug|DrawDebugSphere (Utilities|Array|Get(acopy) (Variables|/Script/OurHome.PlanetActor|GetDrawTerrainVertices _planetactor) (.VerticeIndex (Utilities|Struct|BreakHexGridInfo _returnvalue_3))) 5.0 12 "(R=1.000000,G=0.000000,B=0.000000,A=1.000000)" 9e+01)
          (Development|PrintString (Utilities|String|ToString(Text) (Utilities|Text|FormatText "{0}:{1}:{2}" (Utilities|String|ToString(Integer) (Utilities|Array|Get(acopy) (.HexLocations (Utilities|Struct|BreakHexGridInfo _returnvalue_3)))) (Utilities|String|ToString(Float) (.TerrainHeight (Utilities|Struct|BreakHexGridInfo _returnvalue_3))) (Utilities|String|ToString(Vector) (Utilities|Array|Get(acopy) (Variables|/Script/OurHome.PlanetActor|GetDrawTerrainVertices _planetactor) (.VerticeIndex (Utilities|Struct|BreakHexGridInfo _returnvalue_3)))))) true true "(R=0.000000,G=0.660000,B=1.000000,A=1.000000)" 1e+01)
          (Utilities|FlowControl|Delay 0.2)
          (goto _label Reset)))
      (:Out%201
        (bind _outhit_2 (Collision|LineTraceByChannel _worldlocation_2 (+ _worldlocation_2 (* _worlddirection_2 (Math|Vector|VectorLength _worldlocation_2))) "TraceTypeQuery1" false 0 "None"))
        (if (.bBlockingHit (Collision|BreakHitResult _outhit_2))
          (Class|PlayerCameraPawn|MovePoint (* (Math|Vector|Normalize (.ImpactPoint (Collision|BreakHitResult _outhit_2)) 1e-06) (+ (Class|PlanetActor|GetTerrainHeight (Variables|Default|GetPlanetActor) (Math|Vector|Normalize (.ImpactPoint (Collision|BreakHitResult _outhit_2)) 1e-06)) 2e+02))))))))

(fn ConstructionScript)